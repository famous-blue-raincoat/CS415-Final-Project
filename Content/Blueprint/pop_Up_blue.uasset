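; pop_Up_blue is a trap-like actor that launches a Popup_projectile when the player comes near.
; On BeginPlay it applies its default tile map to a Paper2D tile map component.
; A BP_Player overlapping the sphere triggers Fire, which waits a configurable delay, then spawns the projectile at the Scene component's world transform with itself as owner.
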(event OnComponentBeginOverlap(Sphere)
  (params (OverlappedComponent :type Primitive%20Component%20Object%20Reference) (OtherActor :type Actor%20Object%20Reference) (OtherComp :type Primitive%20Component%20Object%20Reference) (OtherBodyIndex :type Integer) (bFromSweep :type Boolean) (SweepResult :type Hit%20Result%20Structure%20%28by%20ref%29))
  (Utilities|Casting|CastToBP_Player OtherActor)
  (CallFunction|Fire))

(event Custom|Fire
  (Utilities|FlowControl|Delay (Variables|Default|GetDuration))
  (Game|SpawnActorfromClass "/Game/Blueprint/popup_projectile.popup_projectile_C" (Transformation|GetWorldTransform (Variables|Default|GetScene)) "Undefined" self 0))

(event EventBeginPlay
  (Class|PaperTileMapComponent|SetTileMap (Variables|Default|GetPaperTileMap) (Variables|Default|GetDefaultTitlemap)))

(event Collision|EventActorBeginOverlap
  (params (OtherActor :type Actor%20Object%20Reference)))

(event EventTick
  (params (DeltaSeconds :type Float%20%28single-precision%29)))

(fn ConstructionScript)