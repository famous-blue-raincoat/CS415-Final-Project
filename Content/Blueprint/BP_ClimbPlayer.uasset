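; BP_ClimbPlayer is a temporary pawn that the player controls while climbing, moving vertically with the Climb input axis.
; Each tick it compares its height to upper and lower Z targets.
; Past either limit, it teleports itself and BP_Player to the matched top or bottom climb area.
; SwitchPlayer then hides it, possesses BP_Player again and unhides that character.
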(event Custom|SwitchPlayer
  (Rendering|SetActorHiddenInGame true)
  (bind _returnvalue (Actor|GetActorOfClass "/Game/Blueprint/BP_Player.BP_Player_C"))
  (Pawn|Possess (Game|GetPlayerController 0) _returnvalue)
  (Rendering|SetActorHiddenInGame _returnvalue false))

(event EventBeginPlay)

(event Collision|EventActorBeginOverlap
  (params (OtherActor :type Actor%20Object%20Reference)))

(event EventTick
  (params (DeltaSeconds :type Float%20%28single-precision%29))
  (bind _returnvalue (Transformation|GetActorLocation))
  (bind _matchedbottomclimbarea (Variables|Default|GetMatchedBottomClimbArea))
  (bind _matchedtopclimbarea (Variables|Default|GetMatchedTopClimbArea))
  (bind _returnvalue_2 (Transformation|GetActorLocation _matchedtopclimbarea))
  (bind _returnvalue_3 (Transformation|GetActorLocation _matchedbottomclimbarea))
  (bind _z (Math|Vector|BreakVector _returnvalue))
  (if (> _z (Variables|Default|GetTargetUPZ))
    (Transformation|SetActorLocation _returnvalue_2 false false)
    (bind _returnvalue_4 (Actor|GetActorOfClass "/Game/Blueprint/BP_Player.BP_Player_C"))
    (Transformation|SetActorLocation _returnvalue_4 _returnvalue_2 false true)
    (CallFunction|SwitchPlayer)
    (elif (< _z (Variables|Default|GetTargetDownZ))
      (Transformation|SetActorLocation _returnvalue_3 false false)
      (bind _returnvalue_5 (Actor|GetActorOfClass "/Game/Blueprint/BP_Player.BP_Player_C"))
      (Transformation|SetActorLocation _returnvalue_5 _returnvalue_3 false true)
      (CallFunction|SwitchPlayer))))

(event Input|AxisEvents|InputAxisClimb
  (params (AxisValue :type Float%20%28single-precision%29))
  (Transformation|AddActorWorldOffset (Math|Vector|MakeVector 0.0 0.0 (* AxisValue 2.0))))

(fn ConstructionScript)