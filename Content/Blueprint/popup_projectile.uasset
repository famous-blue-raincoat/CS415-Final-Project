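; Side-scroller hazard projectile that damages the player when its Sphere overlaps BP_Player.
; On overlap it plays an explosion sound, triggers the player's DamageScreen and subtracts a fixed amount from the clamped Health stored in GM_SideScroller.
; After a short delay it destroys itself, then calls the game mode's Lose if Health is depleted.
; The graph contains no movement or spawning logic.
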(event OnComponentBeginOverlap(Sphere)
  (params (OverlappedComponent :type Primitive%20Component%20Object%20Reference) (OtherActor :type Actor%20Object%20Reference) (OtherComp :type Primitive%20Component%20Object%20Reference) (OtherBodyIndex :type Integer) (bFromSweep :type Boolean) (SweepResult :type Hit%20Result%20Structure%20%28by%20ref%29))
  (bind _returnvalue (Game|GetGameMode))
  (bind _asgm_side_scroller (Utilities|Casting|CastToGM_SideScroller _returnvalue))
  (bind _asbp_player (Utilities|Casting|CastToBP_Player OtherActor))
  (Audio|PlaySound2D "/Game/Wav/mixkit-explosion-with-rocks-debris-1703.mixkit-explosion-with-rocks-debris-1703" 1.0 1.0 0.0 0 0)
  (Default|DamageScreen _asbp_player)
  (bind _output_get (Variables|/Game/Blueprint/GM_SideScroller.GM_SideScroller_C|SetHealth _asgm_side_scroller (Math|Float|Clamp(Float) (- (Variables|/Game/Blueprint/GM_SideScroller.GM_SideScroller_C|GetHealth _asgm_side_scroller) 2e+01) 0.0 1e+02)))
  (Utilities|FlowControl|Delay 0.2)
  (Actor|DestroyActor)
  (if (<= _output_get 0.0)
    (Default|Lose _asgm_side_scroller)))

(event EventBeginPlay)

(event Collision|EventActorBeginOverlap
  (params (OtherActor :type Actor%20Object%20Reference)))

(event EventTick
  (params (DeltaSeconds :type Float%20%28single-precision%29)))

(fn ConstructionScript)