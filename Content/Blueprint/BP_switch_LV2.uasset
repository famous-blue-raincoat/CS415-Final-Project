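; BP_switch_LV2 is a switch, apparently for level 2 by its name, that BP_Player operates with the Up key while inside its Box trigger.
; Box overlap begin and end enable and disable the actor's input for player controller 0.
; Each Up press adds three Paper tile map components, then destroys the BP_SwitchOFF actor found by class lookup, with no guard against repeated presses.
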(event OnComponentBeginOverlap(Box)
  (params (OverlappedComponent :type Primitive%20Component%20Object%20Reference) (OtherActor :type Actor%20Object%20Reference) (OtherComp :type Primitive%20Component%20Object%20Reference) (OtherBodyIndex :type Integer) (bFromSweep :type Boolean) (SweepResult :type Hit%20Result%20Structure%20%28by%20ref%29))
  (Utilities|Casting|CastToBP_Player OtherActor)
  (Input|EnableInput (Game|GetPlayerController 0)))

(event OnComponentEndOverlap(Box)
  (params (OverlappedComponent :type Primitive%20Component%20Object%20Reference) (OtherActor :type Actor%20Object%20Reference) (OtherComp :type Primitive%20Component%20Object%20Reference) (OtherBodyIndex :type Integer))
  (Utilities|Casting|CastToBP_Player OtherActor)
  (Input|DisableInput (Game|GetPlayerController 0)))

(event EventBeginPlay)

(event Collision|EventActorBeginOverlap
  (params (OtherActor :type Actor%20Object%20Reference)))

(event EventTick
  (params (DeltaSeconds :type Float%20%28single-precision%29)))

(event Input|KeyboardEvents|Up
  (params (Key :type Key%20Structure :default "None"))
  (:Pressed
    (AddComponent|AddPaperTileMapComponent false)
    (AddComponent|AddPaperTileMapComponent false)
    (AddComponent|AddPaperTileMapComponent false)
    (bind _returnvalue (Actor|GetActorOfClass "/Game/Blueprint/BP_SwitchOFF.BP_SwitchOFF_C"))
    (Utilities|IsValid _returnvalue
      (:Is%20Valid
        (Actor|DestroyActor _returnvalue)))))

(fn ConstructionScript)